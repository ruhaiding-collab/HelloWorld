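; Game mode for a timed boba delivery game that tracks score, player level, delivery count and game-over state.
; StartGame resets state on BeginPlay and starts a looping one-second countdown that ends the game at zero.
; BobaDelivered awards level-scaled points, adding time and a capped level every third delivery.
; PackageStall grants bonuses after three deliveries, and MaxScore_Event sets game over at a score threshold; neither is called here.
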(event Custom|Clock_Event
  (bind _output_get (Variables|Default|SetTime (- (Variables|Default|GetTime) 1)))
  (if (== _output_get 0)
    (Variables|Default|SetGameOver true)
    (Utilities|Time|ClearTimerbyFunctionName 0 "Clock_Event")))

(event Custom|MaxScore_Event
  (bind _output_get (Variables|Default|SetScore (Variables|Default|GetScore)))
  (if (>= _output_get 100)
    (Variables|Default|SetGameOver true)))

(event EventBeginPlay
  (Utilities|StartGame))

(fn ConstructionScript)

(fn BobaDelivered
  (Variables|Default|SetScore (+ (Variables|Default|GetScore) (* (Variables|Default|GetPlayerLevel) 10)))
  (bind _output_get (Variables|Default|SetDeliveryCount (+ (Variables|Default|GetDeliveryCount) 1)))
  (if (== (Math|Integer|%(Integer) _output_get 3) 0)
    (Variables|Default|SetTime (+ (Variables|Default|GetTime) 5))
    (Variables|Default|SetPlayerLevel (Math|Integer|Min(Integer) (+ (Variables|Default|GetPlayerLevel) 1) 5))))

(fn PackageStall
  (bind _output_get (Variables|Default|SetDeliveryCount (Variables|Default|GetDeliveryCount)))
  (if (>= _output_get 3)
    (Variables|Default|SetTime (+ (Variables|Default|GetTime) 10))
    (Variables|Default|SetScore (+ (* (Variables|Default|GetPlayerLevel) 20) (Variables|Default|GetScore)))))