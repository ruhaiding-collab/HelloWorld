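; BP_Boba is a pickup that jumps around the play area until the player collects it.
; InitialBoba teleports it to a random point at fixed height, then re-arms its own timer with a delay that shrinks as the GameMode's PlayerLevel rises.
; Player overlap, while the game is not over, notifies BP_GameMode of delivery, destroys the boba and spawns a base Actor class at its transform.
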(event EventBeginPlay
  (bind _asbp_game_mode (Utilities|Casting|CastToBP_GameMode (Game|GetGameMode)))
  (Variables|Default|SetGameMode _asbp_game_mode)
  (CallFunction|InitialBoba))

(event Collision|EventActorBeginOverlap
  (params (OtherActor :type Actor%20Object%20Reference))
  (if (and (== OtherActor (Game|GetPlayerCharacter 0)) (not (Variables|/Game/BP_GameMode.BP_GameMode_C|GetGameOver (Variables|Default|GetGameMode))))
    (Default|BobaDelivered (Variables|Default|GetGameMode))
    (Actor|DestroyActor)
    (Game|SpawnActorfromClass "/Script/Engine.Actor" (Transformation|GetActorTransform) "Undefined" "MultiplyWithRoot" 0 0)))

(event EventTick
  (params (DeltaSeconds :type Float%20%28single-precision%29)))

(fn ConstructionScript)

(fn InitialBoba
  (Transformation|Teleport (Math|Vector|MakeVector (Math|Random|RandomFloatinRange 1e+02 2.8e+03) (Math|Random|RandomFloatinRange 1.4e+02 3.3e+03) 1.3e+02) "0, 0, 0")
  (Utilities|Time|SetTimerbyFunctionName 0 "InitialBoba" (Math|Conversions|ToFloat(Integer) (- 10 (Variables|/Game/BP_GameMode.BP_GameMode_C|GetPlayerLevel (Variables|Default|GetGameMode))))))