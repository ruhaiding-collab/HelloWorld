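; BP_Stall is a trigger actor that reports to the game mode when the player reaches a stall.
; It caches BP_GameMode on BeginPlay.
; When the player character begins overlapping it and the game is not over, it calls the game mode's PackageStall, gated by a DoOnce with no reset so each stall fires only once.
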(event EventBeginPlay
  (bind _asbp_game_mode (Utilities|Casting|CastToBP_GameMode (Game|GetGameMode)))
  (Variables|Default|SetGameMode _asbp_game_mode))

(event Collision|EventActorBeginOverlap
  (params (OtherActor :type Actor%20Object%20Reference))
  (if (and (== OtherActor (Game|GetPlayerCharacter 0)) (not (Variables|/Game/BP_GameMode.BP_GameMode_C|GetGameOver (Variables|Default|GetGameMode))))
    (Utilities|FlowControl|DoOnce false
      (:Completed
        (Default|PackageStall (Variables|Default|GetGameMode))))))

(event EventTick
  (params (DeltaSeconds :type Float%20%28single-precision%29)))

(fn ConstructionScript)